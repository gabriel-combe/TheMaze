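; MyDoorObject is an interactable door that displays its required key on a widget component, coloured by door tier.
; Shortly after BeginPlay it caches the W_DoorText widget, sets the key text and picks a Common, Uncommon or Rare colour.
; Interact defers to the parent implementation, then refreshes the text, with a manual render update requested after each widget change.
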(event `self.ReceiveBeginPlay`
  (`KismetSystemLibrary.Delay` 0.2)
  (bind _asw_door_text (cast `/Game/HUD/W_DoorText` (`WidgetComponent.GetUserWidgetObject` (`self.WidgetDoor`))))
  (bind _output_get (set `self.As W Door Text` _asw_door_text))
  (`/Game/HUD/W_DoorText.SetDoorText` _output_get (`self.RequiredKey`))
  (`/Game/HUD/W_DoorText.SetColour` (`self.As W Door Text`) (select `EKeyDoorTier` (`self.DoorTier`) :`KeyDoor_Common` (struct :`R` 1.0 :`G` 1.0 :`B` 1.0 :`A` 1.0) :`KeyDoor_Uncommon` (struct :`R` 0.019608 :`G` 0.423529 :`B` 0.117647 :`A` 1.0) :`KeyDoor_Rare` (struct :`R` 0.52549 :`G` 0.039216 :`B` 0.023529 :`A` 1.0) :!type "LinearColor Structure"))
  (`WidgetComponent.RequestRenderUpdate` (`self.WidgetDoor`)))

(event `self.Interact`
  (params (player :type "TheMazeCharacter Object Reference"))
  (`parent.Interact` player)
  (`/Game/HUD/W_DoorText.SetDoorText` (`self.As W Door Text`) (`self.RequiredKey`))
  (`WidgetComponent.RequestRenderUpdate` (`self.WidgetDoor`)))

(fn `UserConstructionScript`)